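; BP_Dropper is a chopstick-holding skeletal character that alternates between eating and dropping Pickup actors, with its Karaage mesh initially hidden.
; A randomized timer calls StartDrop, which plays the drop montage if IsTryDrop is set, clearing it, or else the eat montage.
; Drop spawns a pickup at the Arrow and launches it with a randomized forward-based impulse.
; Drop and EatEnd, not called within these graphs, re-arm the timer while looping.
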(fn `Drop`
  (bind _returnvalue (* (`SceneComponent.GetForwardVector` (`self.Arrow`)) (`KismetMathLibrary.MakeVector` (`KismetMathLibrary.RandomFloat`) (`KismetMathLibrary.RandomFloat`) (`KismetMathLibrary.RandomFloat`))))
  (bind _returnvalue_2 (`|SpawnActorFromClass` "/Game/Blueprints/Pickup.Pickup_C" (`KismetMathLibrary.MakeTransform` (`SceneComponent.K2_GetComponentLocation` (`self.Arrow`)) (struct) (1.0 1.0 1.0)) "Undefined" "OverrideRootScale"))
  (`SceneComponent.K2_SetWorldRotation` (`self.Arrow1`) (`KismetMathLibrary.MakeRotationFromAxes` _returnvalue) false false)
  (`PrimitiveComponent.AddImpulse` (`/Game/Blueprints/Pickup.StaticMesh` _returnvalue_2) (* _returnvalue 500.0) "None" true)
  (if (`self.Loop`)
    (`self.SetTimer`)))

(fn `EatEnd`
  (if (`self.Loop`)
    (`self.SetTimer`)))

(fn `SetTimer`
  (set `self.Loop` true)
  (`KismetSystemLibrary.K2_SetTimer` null "StartDrop" (`KismetMathLibrary.Lerp` (`self.minInterval`) (`self.maxInterval`) (`KismetMathLibrary.RandomFloat`))))

(fn `StartDrop`
  (bind _returnvalue (`SkeletalMeshComponent.GetAnimInstance` (`self.SkeletalMesh`)))
  (if (`self.IsTryDrop`)
    (set `self.IsTryDrop` false)
    (`AnimInstance.Montage_Play` _returnvalue (`self.DropMontage`) 1.0 "MontageLength" 0.0)
    (else
      (`AnimInstance.Montage_Play` _returnvalue (`self.EatMontage`) 1.0 "MontageLength" 0.0))))

(fn `UserConstructionScript`
  (`SceneComponent.K2_AttachToComponent` (`self.Chopstick`) (`self.SkeletalMesh`) "Chopskick" "KeepRelative" "KeepRelative" "KeepWorld" true)
  (`SceneComponent.SetVisibility` (`self.karaage`) false false))