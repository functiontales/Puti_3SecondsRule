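; Pickup actor that removes itself a set time after it lands on the ground.
; The first static mesh hit against BP_AreaGround marks it dropped, resets PassingTime and starts a DestroyTime timer that calls Destroy.
; While dropped, Tick accumulates PassingTime, though this graph never reads it for other logic.
; The Destroyed event clears and invalidates the timer handle.
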(event `self.StaticMesh.OnComponentHit`
  (params (HitComponent :type "PrimitiveComponent Object Reference") (OtherActor :type "Actor Object Reference") (OtherComp :type "PrimitiveComponent Object Reference") (NormalImpulse :type "Vector Structure") (Hit :type "HitResult Structure (by ref)"))
  (if (not (`self.IsDropped`))
    (cast `/Game/Blueprints/BP_AreaGround` OtherActor)
    (`/Engine/EditorBlueprintResources/StandardMacros.DoOnce` false
      (:`Completed`
        (set `self.IsDropped` true)
        (set `self.PassingTime` 0.0)
        (bind _returnvalue (`KismetSystemLibrary.K2_SetTimer` null "Destroy" (`self.DestroyTime`)))
        (set `self.DestoryHandeTimer` _returnvalue)))))

(event `self.ReceiveTick`
  (params (DeltaSeconds :type "Float (single-precision)"))
  (if (`self.IsDropped`)
    (set `self.PassingTime` (+ DeltaSeconds (`self.PassingTime`)))))

(event `self.ReceiveDestroyed`
  (`KismetSystemLibrary.K2_ClearAndInvalidateTimerHandle` (`self.DestoryHandeTimer`)))

(fn `Destroy`
  (`self.K2_DestroyActor`))

(fn `UserConstructionScript`)