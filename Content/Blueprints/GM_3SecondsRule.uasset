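; Game mode for a "3 Seconds Rule" game that constantly drains the player's life and runs a one-minute countdown.
; Tick lazily caches the BP_MainCharacter pawn, applies decay scaled by initial life while life is non-negative, and updates the remaining time.
; The timer's GameOver event is empty, and the state functions are stubs: SetCurrentState always forwards Playing to a switch with no branches.
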(event `self.ReceiveBeginPlay`
  (bind _returnvalue (`KismetSystemLibrary.K2_SetTimerDelegate` (delegate `GameOver`) 60.0))
  (set `self.RemainingTimer` _returnvalue))

(event `GameOver`)

(event `self.ReceiveTick`
  (params (DeltaSeconds :type "Float (single-precision)"))
  (bind _player (`self.Player`))
  (`|ExecutionSequence`
    (:`then_0`
      (`/Engine/EditorBlueprintResources/StandardMacros.IsValid` (`self.Player`)
        (:`Is Valid`
          _)
        (:`Is Not Valid`
          (bind _asbp_main_character (cast `/Game/Blueprints/BP_MainCharacter` (`GameplayStatics.GetPlayerPawn` 0)))
          (set `self.Player` _asbp_main_character)))
      (if (>= (`/Game/Blueprints/BP_MainCharacter.Life` _player) 0.0)
        (`/Game/Blueprints/BP_MainCharacter.UpdateLife` _player (* (* (* DeltaSeconds -1.0) (`self.DecayRate`)) (`/Game/Blueprints/BP_MainCharacter.InitialLife` _player)))))
    (:`then_1`
      (set `self.RemainingTime` (`KismetSystemLibrary.K2_GetTimerRemainingTimeHandle` (`self.RemainingTimer`))))))

(fn `HandleNewState`
  (params (NewParam :type "/Game/Blueprints/GamePlayState Enum"))
  (bind _output_get (set `self.CurrentState` NewParam))
  (switch `/Game/Blueprints/GamePlayState` _output_get))

(fn `SetCurrentState`
  (params (NewParam :type "/Game/Blueprints/GamePlayState Enum"))
  (set `self.CurrentState` NewParam)
  (`self.HandleNewState` "NewEnumerator0"))

(fn `UserConstructionScript`)