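; BP_3SecPC is the player controller for a three-second-rule pickup game, tracking Life, Satiation and collected pickups.
; BeginPlay adds the main HUD and disables pawn input until the gamepad Special Right button enables it once and sets Ready; Q quits.
; Pickuped adjusts life, plays a success or failure sound based on elapsed time, and weakens the pawn when late.
; Every pickup raises the count and satiation, then updates the pawn's speed.
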(event `self.ReceiveBeginPlay`
  (bind _returnvalue (`|CreateWidget` "/Game/HUD/WB_MainHUD.WB_MainHUD_C"))
  (bind _output_get (set `self.HUDReference` _returnvalue))
  (`UserWidget.AddToViewport` _output_get 0)
  (bind _asbp_main_character (cast `/Game/Blueprints/BP_MainCharacter` (`GameplayStatics.GetPlayerPawn` 0)))
  (bind _output_get_2 (set `self.PlayerPawnReference` _asbp_main_character))
  (`self.DisableInput` _output_get_2 self))

(event `Key|Gamepad_Special_Right`
  (params (Key :type "Key Structure" :default "AnyKey"))
  (bind _playerpawnreference (`self.PlayerPawnReference`))
  (:`Pressed`
    (`/Engine/EditorBlueprintResources/StandardMacros.IsValid` _playerpawnreference
      (:`Is Valid`
        (`/Engine/EditorBlueprintResources/StandardMacros.DoOnce` false
          (:`Completed`
            (`self.EnableInput` _playerpawnreference self)
            (set `self.Ready?` true)))))))

(event `Key|Q`
  (params (Key :type "Key Structure" :default "AnyKey"))
  (:`Pressed`
    (`KismetSystemLibrary.QuitGame` null "Quit")))

(fn `Pickuped`
  (params (PickupPassingTime :type "Float (double-precision)"))
  (bind _playerpawnreference (`self.PlayerPawnReference`))
  (bind _returnvalue (`self.K2_GetActorLocation` (`self.PlayerPawnReference`)))
  (if (<= PickupPassingTime 3.0)
    (`self.UpdateLife` (`self.PickupRecover`))
    (`GameplayStatics.SpawnSoundAtLocation` "/Game/Audio/Puti_3secRuleSuccess_Cue.Puti_3secRuleSuccess_Cue" _returnvalue)
    (else
      (`self.UpdateLife` (`self.PickupDamage`))
      (`GameplayStatics.SpawnSoundAtLocation` "/Game/Audio/Puti_3secRuleFailed_Cue.Puti_3secRuleFailed_Cue" _returnvalue)
      (`/Game/Blueprints/BP_MainCharacter.Weaken` _playerpawnreference)))
  (`/Engine/EditorBlueprintResources/StandardMacros.IncrementInt` (`self.CollectedPickup`)
    (:`  `
      (set `self.Satiation` (+ (`self.Satiation`) 1.0))
      (`/Game/Blueprints/BP_MainCharacter.UpdateSpeed` _playerpawnreference))))

(fn `UpdateLife`
  (params (NewParam :type "Float (double-precision)"))
  (set `self.Life` (+ NewParam (`self.Life`))))

(fn `UpdateSatiation`
  (params (NewParam :type "Float (double-precision)"))
  (set `self.Satiation` (+ NewParam (`self.Satiation`))))

(fn `UserConstructionScript`)